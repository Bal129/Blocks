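; BP_AssemblyManager tracks how many blocks are attached in an assembly game and handles the win state.
; Increment and decrement functions update the count and recolor the block's image in the WB_ProgressChecker widget, green or faded red, using BlockGroup to pick the canvas and BlockId as child index.
; CheckWinning compares the count to the total and, on a match, plays a sound, shows WB_GameWin with the cursor and pauses the game.
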(fn ConstructionScript)

(fn CheckWinning
  (bind _returnvalue (Game|GetPlayerController 0))
  (if (== (Variables|Default|GettotalNumBlocks) (Variables|Default|GetnumBlocks))
    ;[1 1 1] Open Game Win Widget
    (bind _returnvalue_2 (UserInterface|CreateWidget "/Game/UI/WB_GameWin.WB_GameWin_C" _returnvalue))
    (Audio|PlaySound2D "/Game/Audio/SFX/win.win" 1.0 1.0 0.0 0 0)
    (UserInterface|Viewport|AddtoViewport _returnvalue_2 0)
    (Input|SetInputModeGameandUI _returnvalue _returnvalue_2 "DoNotLock" true false)
    (Variables|/Script/Engine.PlayerController|SetbShowMouseCursor _returnvalue true)
    (Game|SetGamePaused true)))

(fn IncrementNumBlocks
  (params (blockId :type Integer) (blockGroup :type Integer))
  (Variables|Default|SetnumBlocks (+ (Variables|Default|GetnumBlocks) 1))
  (bind _foundwidgets (Widget|GetAllWidgetsOfClass "/Game/UI/WB_ProgressChecker.WB_ProgressChecker_C" false))
  (switch int blockGroup
    (:0
      (Variables|Default|SetcurrentCPanel (Variables|/Game/UI/WB_ProgressChecker.WB_ProgressChecker_C|GetCanvas_M1 (Utilities|Array|Get(acopy) _foundwidgets))))
    (:1
      (Variables|Default|SetcurrentCPanel (Variables|/Game/UI/WB_ProgressChecker.WB_ProgressChecker_C|GetCanvas_M2 (Utilities|Array|Get(acopy) _foundwidgets))))
    (:2
      (Variables|Default|SetcurrentCPanel (Variables|/Game/UI/WB_ProgressChecker.WB_ProgressChecker_C|GetCanvas_U (Utilities|Array|Get(acopy) _foundwidgets)))))
  (bind _asimage (Utilities|Casting|CastToImage (Class|PanelWidget|GetChildat (Variables|Default|GetcurrentCPanel) blockId)))
  (Variables|/Script/UMG.Image|SetColorAndOpacity _asimage (Math|Color|MakeColor 0.0 1.0 0.0 0.8)))

(fn DecrementNumBlocks
  (params (blockId :type Integer) (blockGroup :type Integer))
  (Variables|Default|SetnumBlocks (- (Variables|Default|GetnumBlocks) 1))
  (bind _foundwidgets (Widget|GetAllWidgetsOfClass "/Game/UI/WB_ProgressChecker.WB_ProgressChecker_C" false))
  (switch int blockGroup
    (:0
      (Variables|Default|SetcurrentCPanel (Variables|/Game/UI/WB_ProgressChecker.WB_ProgressChecker_C|GetCanvas_M1 (Utilities|Array|Get(acopy) _foundwidgets))))
    (:1
      (Variables|Default|SetcurrentCPanel (Variables|/Game/UI/WB_ProgressChecker.WB_ProgressChecker_C|GetCanvas_M2 (Utilities|Array|Get(acopy) _foundwidgets))))
    (:2
      (Variables|Default|SetcurrentCPanel (Variables|/Game/UI/WB_ProgressChecker.WB_ProgressChecker_C|GetCanvas_U (Utilities|Array|Get(acopy) _foundwidgets)))))
  (bind _asimage (Utilities|Casting|CastToImage (Class|PanelWidget|GetChildat (Variables|Default|GetcurrentCPanel) blockId)))
  (Variables|/Script/UMG.Image|SetColorAndOpacity _asimage (Math|Color|MakeColor 1.0 0.0 0.0 0.3)))