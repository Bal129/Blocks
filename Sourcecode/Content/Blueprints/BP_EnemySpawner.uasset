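; Enemy spawner zone that periodically spawns BP_Enemy actors while the first-person player is inside its sphere.
; Overlap begin shows a zone warning on the WP_HealthBar widget and starts a looping one-second timer; overlap end clears both.
; Each spawn picks a random reachable nav point around the spawner and passes SpawnerType to the enemy.
; On BeginPlay, SpawnerType also selects the pillar's material.
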(event OnComponentBeginOverlap(Sphere)
  (params (OverlappedComponent :type Primitive%20Component%20Object%20Reference) (OtherActor :type Actor%20Object%20Reference) (OtherComp :type Primitive%20Component%20Object%20Reference) (OtherBodyIndex :type Integer) (bFromSweep :type Boolean) (SweepResult :type Hit%20Result%20Structure%20%28by%20ref%29))
  (bind _asbp_first_person_character (Utilities|Casting|CastToBP_FirstPersonCharacter OtherActor))
  (if (== OtherActor _asbp_first_person_character)
    (bind _foundwidgets (Widget|GetAllWidgetsOfClass "/Game/UI/WP_HealthBar.WP_HealthBar_C" true))
    (Rendering|Components|TextRender|SetText (Variables|/Game/UI/WP_HealthBar.WP_HealthBar_C|GetText_indicator (Utilities|Array|Get(acopy) _foundwidgets)) (Utilities|Text|ToText(String) (Utilities|String|Append (Variables|Default|Getzone) ": Beware of the enemies")))
    (Utilities|Casting|CastToCharacter OtherActor)
    (bind _returnvalue (Utilities|Time|SetTimerbyEvent (delegate Custom|Spawn%20Enemy) 1.0 true))
    (bind _output_get (Variables|Default|SetNewVar _returnvalue))))

(event OnComponentEndOverlap(Sphere)
  (params (OverlappedComponent :type Primitive%20Component%20Object%20Reference) (OtherActor :type Actor%20Object%20Reference) (OtherComp :type Primitive%20Component%20Object%20Reference) (OtherBodyIndex :type Integer))
  (bind _asbp_first_person_character (Utilities|Casting|CastToBP_FirstPersonCharacter OtherActor))
  (if (== OtherActor _asbp_first_person_character)
    (bind _foundwidgets (Widget|GetAllWidgetsOfClass "/Game/UI/WP_HealthBar.WP_HealthBar_C" true))
    (Rendering|Components|TextRender|SetText (Variables|/Game/UI/WP_HealthBar.WP_HealthBar_C|GetText_indicator (Utilities|Array|Get(acopy) _foundwidgets)) (Utilities|Text|ToText(String) ""))
    (Utilities|Casting|CastToCharacter OtherActor)
    (Utilities|Time|ClearandInvalidateTimerbyHandle (stale OnComponentBeginOverlap(Sphere) _output_get))))

(event Custom|Spawn%20Enemy
  (bind _returnvalue (Game|SpawnActorfromClass "/Game/Blueprints/BP_Enemy.BP_Enemy_C" (Math|Transform|MakeTransform (.RandomLocation (AI|Navigation|GetRandomReachablePointinRadius (Transformation|GetActorLocation) 1e+03 0 0)) "0, 0, 0" "1.000000,1.000000,1.000000") "Undefined" "MultiplyWithRoot" 0 0))
  (Variables|/Game/Blueprints/BP_Enemy.BP_Enemy_C|SetspawnerType _returnvalue (Variables|Default|GetspawnerType)))

(event EventBeginPlay
  (bind _pillar (Variables|Default|GetPillar))
  (switch int (Variables|Default|GetspawnerType)
    (:0
      (Rendering|Material|SetMaterial _pillar 0 "/Game/StarterContent/Materials/M_Brick_Clay_Beveled.M_Brick_Clay_Beveled"))
    (:1
      (Rendering|Material|SetMaterial _pillar 0 "/Game/StarterContent/Materials/M_Wood_Floor_Walnut_Worn.M_Wood_Floor_Walnut_Worn"))
    (:2
      (Rendering|Material|SetMaterial _pillar 0 "/Game/StarterContent/Materials/M_Ground_Grass.M_Ground_Grass"))))

(fn ConstructionScript)