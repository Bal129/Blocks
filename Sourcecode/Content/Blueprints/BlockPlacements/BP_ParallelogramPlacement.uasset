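; Placement slot that detects when a parallelogram block of the matching type is correctly placed in an assembly puzzle.
; Collision box overlaps track block counts and type, while eight child point colliders count overlaps to confirm alignment.
; When a single matching block covers all points, UpdateIndicator turns the indicator blue, plays a sound, increments BP_AssemblyManager's count and checks for a win.
; A parallelogram leaving a filled slot decrements that count.
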(event OnComponentBeginOverlap(CoPoint1)
  (params (OverlappedComponent :type Primitive%20Component%20Object%20Reference) (OtherActor :type Actor%20Object%20Reference) (OtherComp :type Primitive%20Component%20Object%20Reference) (OtherBodyIndex :type Integer) (bFromSweep :type Boolean) (SweepResult :type Hit%20Result%20Structure%20%28by%20ref%29))
  ;[1 1 1] Begin Overlap points
  (Variables|Default|SetoverlapPoints (+ (Variables|Default|GetoverlapPoints) 1))
  (CallFunction|UpdateIndicator))

(event OnComponentBeginOverlap(CoPoint2)
  (params (OverlappedComponent :type Primitive%20Component%20Object%20Reference) (OtherActor :type Actor%20Object%20Reference) (OtherComp :type Primitive%20Component%20Object%20Reference) (OtherBodyIndex :type Integer) (bFromSweep :type Boolean) (SweepResult :type Hit%20Result%20Structure%20%28by%20ref%29))
  ;[1 1 1] Begin Overlap points
  (Variables|Default|SetoverlapPoints (+ (Variables|Default|GetoverlapPoints) 1))
  (CallFunction|UpdateIndicator))

(event OnComponentBeginOverlap(CoPoint3)
  (params (OverlappedComponent :type Primitive%20Component%20Object%20Reference) (OtherActor :type Actor%20Object%20Reference) (OtherComp :type Primitive%20Component%20Object%20Reference) (OtherBodyIndex :type Integer) (bFromSweep :type Boolean) (SweepResult :type Hit%20Result%20Structure%20%28by%20ref%29))
  ;[1 1 1] Begin Overlap points
  (Variables|Default|SetoverlapPoints (+ (Variables|Default|GetoverlapPoints) 1))
  (CallFunction|UpdateIndicator))

(event OnComponentBeginOverlap(CoPoint4)
  (params (OverlappedComponent :type Primitive%20Component%20Object%20Reference) (OtherActor :type Actor%20Object%20Reference) (OtherComp :type Primitive%20Component%20Object%20Reference) (OtherBodyIndex :type Integer) (bFromSweep :type Boolean) (SweepResult :type Hit%20Result%20Structure%20%28by%20ref%29))
  ;[1 1 1] Begin Overlap points
  (Variables|Default|SetoverlapPoints (+ (Variables|Default|GetoverlapPoints) 1))
  (CallFunction|UpdateIndicator))

(event OnComponentBeginOverlap(CoPoint5)
  (params (OverlappedComponent :type Primitive%20Component%20Object%20Reference) (OtherActor :type Actor%20Object%20Reference) (OtherComp :type Primitive%20Component%20Object%20Reference) (OtherBodyIndex :type Integer) (bFromSweep :type Boolean) (SweepResult :type Hit%20Result%20Structure%20%28by%20ref%29))
  ;[1 1 1] Begin Overlap points
  (Variables|Default|SetoverlapPoints (+ (Variables|Default|GetoverlapPoints) 1))
  (CallFunction|UpdateIndicator))

(event OnComponentBeginOverlap(Collisionbox)
  (params (OverlappedComponent :type Primitive%20Component%20Object%20Reference) (OtherActor :type Actor%20Object%20Reference) (OtherComp :type Primitive%20Component%20Object%20Reference) (OtherBodyIndex :type Integer) (bFromSweep :type Boolean) (SweepResult :type Hit%20Result%20Structure%20%28by%20ref%29))
  ;[1 1 1] Check when a block enter collision
  (Variables|Default|SettotalBlocks (+ (Variables|Default|GettotalBlocks) 1))
  (CallFunction|UpdateIndicator)
  (bind _asblock_parallelogram (Utilities|Casting|CastToBlock_Parallelogram OtherActor))
  (if (== _asblock_parallelogram OtherActor)
    (Variables|Default|SettotalDesiredBlocks (+ (Variables|Default|GettotalDesiredBlocks) 1))
    (Variables|Default|SetblockType (Variables|/Game/Blueprints/Blocks/Block_Parallelogram.Block_Parallelogram_C|Gettype _asblock_parallelogram))))

(event OnComponentEndOverlap(Collisionbox)
  (params (OverlappedComponent :type Primitive%20Component%20Object%20Reference) (OtherActor :type Actor%20Object%20Reference) (OtherComp :type Primitive%20Component%20Object%20Reference) (OtherBodyIndex :type Integer))
  ;[1 1 1] Check when a block exit collision box
  (Variables|Default|SettotalBlocks (- (Variables|Default|GettotalBlocks) 1))
  (CallFunction|UpdateIndicator)
  (bind _asblock_parallelogram (Utilities|Casting|CastToBlock_Parallelogram OtherActor))
  (if (== _asblock_parallelogram OtherActor)
    (Variables|Default|SettotalDesiredBlocks (- (Variables|Default|GettotalDesiredBlocks) 1))
    (if (Variables|Default|GetcontainsBlock)
      (Variables|Default|SetcontainsBlock false)
      (Default|DecrementNumBlocks (Variables|Default|GetassemblyManager) (Variables|Default|GetblockPosition) (Variables|Default|GetblockGroup)))))

(event OnComponentBeginOverlap(CoPoint6)
  (params (OverlappedComponent :type Primitive%20Component%20Object%20Reference) (OtherActor :type Actor%20Object%20Reference) (OtherComp :type Primitive%20Component%20Object%20Reference) (OtherBodyIndex :type Integer) (bFromSweep :type Boolean) (SweepResult :type Hit%20Result%20Structure%20%28by%20ref%29))
  ;[1 1 1] Begin Overlap points
  (Variables|Default|SetoverlapPoints (+ (Variables|Default|GetoverlapPoints) 1))
  (CallFunction|UpdateIndicator))

(event OnComponentEndOverlap(CoPoint1)
  (params (OverlappedComponent :type Primitive%20Component%20Object%20Reference) (OtherActor :type Actor%20Object%20Reference) (OtherComp :type Primitive%20Component%20Object%20Reference) (OtherBodyIndex :type Integer))
  ;[1 1 1] End Overlap points
  (Variables|Default|SetoverlapPoints (- (Variables|Default|GetoverlapPoints) 1))
  (CallFunction|UpdateIndicator))

(event OnComponentEndOverlap(CoPoint2)
  (params (OverlappedComponent :type Primitive%20Component%20Object%20Reference) (OtherActor :type Actor%20Object%20Reference) (OtherComp :type Primitive%20Component%20Object%20Reference) (OtherBodyIndex :type Integer))
  ;[1 1 1] End Overlap points
  (Variables|Default|SetoverlapPoints (- (Variables|Default|GetoverlapPoints) 1))
  (CallFunction|UpdateIndicator))

(event OnComponentBeginOverlap(CoPoint7)
  (params (OverlappedComponent :type Primitive%20Component%20Object%20Reference) (OtherActor :type Actor%20Object%20Reference) (OtherComp :type Primitive%20Component%20Object%20Reference) (OtherBodyIndex :type Integer) (bFromSweep :type Boolean) (SweepResult :type Hit%20Result%20Structure%20%28by%20ref%29))
  ;[1 1 1] Begin Overlap points
  (Variables|Default|SetoverlapPoints (+ (Variables|Default|GetoverlapPoints) 1))
  (CallFunction|UpdateIndicator))

(event OnComponentEndOverlap(CoPoint3)
  (params (OverlappedComponent :type Primitive%20Component%20Object%20Reference) (OtherActor :type Actor%20Object%20Reference) (OtherComp :type Primitive%20Component%20Object%20Reference) (OtherBodyIndex :type Integer))
  ;[1 1 1] End Overlap points
  (Variables|Default|SetoverlapPoints (- (Variables|Default|GetoverlapPoints) 1))
  (CallFunction|UpdateIndicator))

(event OnComponentEndOverlap(CoPoint4)
  (params (OverlappedComponent :type Primitive%20Component%20Object%20Reference) (OtherActor :type Actor%20Object%20Reference) (OtherComp :type Primitive%20Component%20Object%20Reference) (OtherBodyIndex :type Integer))
  ;[1 1 1] End Overlap points
  (Variables|Default|SetoverlapPoints (- (Variables|Default|GetoverlapPoints) 1))
  (CallFunction|UpdateIndicator))

(event OnComponentEndOverlap(CoPoint5)
  (params (OverlappedComponent :type Primitive%20Component%20Object%20Reference) (OtherActor :type Actor%20Object%20Reference) (OtherComp :type Primitive%20Component%20Object%20Reference) (OtherBodyIndex :type Integer))
  ;[1 1 1] End Overlap points
  (Variables|Default|SetoverlapPoints (- (Variables|Default|GetoverlapPoints) 1))
  (CallFunction|UpdateIndicator))

(event OnComponentEndOverlap(CoPoint6)
  (params (OverlappedComponent :type Primitive%20Component%20Object%20Reference) (OtherActor :type Actor%20Object%20Reference) (OtherComp :type Primitive%20Component%20Object%20Reference) (OtherBodyIndex :type Integer))
  ;[1 1 1] End Overlap points
  (Variables|Default|SetoverlapPoints (- (Variables|Default|GetoverlapPoints) 1))
  (CallFunction|UpdateIndicator))

(event OnComponentEndOverlap(CoPoint7)
  (params (OverlappedComponent :type Primitive%20Component%20Object%20Reference) (OtherActor :type Actor%20Object%20Reference) (OtherComp :type Primitive%20Component%20Object%20Reference) (OtherBodyIndex :type Integer))
  ;[1 1 1] End Overlap points
  (Variables|Default|SetoverlapPoints (- (Variables|Default|GetoverlapPoints) 1))
  (CallFunction|UpdateIndicator))

(event OnComponentEndOverlap(CoPoint8)
  (params (OverlappedComponent :type Primitive%20Component%20Object%20Reference) (OtherActor :type Actor%20Object%20Reference) (OtherComp :type Primitive%20Component%20Object%20Reference) (OtherBodyIndex :type Integer))
  ;[1 1 1] End Overlap points
  (Variables|Default|SetoverlapPoints (- (Variables|Default|GetoverlapPoints) 1))
  (CallFunction|UpdateIndicator))

(event OnComponentBeginOverlap(CoPoint8)
  (params (OverlappedComponent :type Primitive%20Component%20Object%20Reference) (OtherActor :type Actor%20Object%20Reference) (OtherComp :type Primitive%20Component%20Object%20Reference) (OtherBodyIndex :type Integer) (bFromSweep :type Boolean) (SweepResult :type Hit%20Result%20Structure%20%28by%20ref%29))
  ;[1 1 1] Begin Overlap points
  (Variables|Default|SetoverlapPoints (+ (Variables|Default|GetoverlapPoints) 1))
  (CallFunction|UpdateIndicator))

(event EventBeginPlay
  ;[1 1 1] Set the desired overlapped points
  (Utilities|FlowControl|Sequence
    (:then_0
      (Variables|Default|SetdesiredOverlapPoints (Class|SceneComponent|GetNumChildrenComponents (Variables|Default|GetCollision%20box))))
    (:then_1
      (bind _returnvalue (Actor|GetActorOfClass "/Game/Blueprints/BP_AssemblyManager.BP_AssemblyManager_C"))
      (Variables|Default|SetassemblyManager _returnvalue))))

(fn ConstructionScript)

(fn UpdateIndicator
  (bind _indicator (Variables|Default|GetIndicator))
  (bind _assemblymanager (Variables|Default|GetassemblyManager))
  ;[1 1 1] Set indicator to different material when conditions met
  (if (Math|Boolean|ANDBoolean (== (Variables|Default|GettotalBlocks) 1) (== (Variables|Default|GettotalDesiredBlocks) 1) (>= (Variables|Default|GetoverlapPoints) (Variables|Default|GetdesiredOverlapPoints)) (== (Variables|Default|GetplacementType) (Variables|Default|GetblockType)))
    (Rendering|Material|SetMaterial _indicator 0 "/Game/LevelPrototyping/Materials/MI_Solid_Blue.MI_Solid_Blue")
    (if (not (Variables|Default|GetcontainsBlock))
      (Variables|Default|SetcontainsBlock true)
      (Audio|PlaySound2D "/Game/Audio/SFX/progress.progress" 1.0 1.0 0.0 0 0)
      (Default|IncrementNumBlocks _assemblymanager (Variables|Default|GetblockPosition) (Variables|Default|GetblockGroup))
      (Default|CheckWinning _assemblymanager))
    (else
      (Rendering|Material|SetMaterial _indicator 0 "/Game/FPWeapon/Materials/BaseMaterial.BaseMaterial"))))