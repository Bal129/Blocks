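; Melee enemy that chases the player on sight, attacks with a punch montage and drops a random block when killed by impact.
; PawnSensing starts an AI MoveTo; Tick halts movement until the player has been seen.
; Fast non-player components overlapping the capsule inflict self-damage; lethal hits spawn one of four block shapes at a floor trace, with material set from SpawnerType.
; Capsule hits launch the player away.
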(event OnSeePawn(PawnSensing)
  (params (Pawn :type Pawn%20Object%20Reference))
  ;[1 1 1] Enemy Follow Algorithm
  (Variables|Default|SetisSeeingPlayer? true)
  (CallFunction|FollowPlayer))

(event OnComponentHit(CapsuleComponent)
  (params (HitComponent :type Primitive%20Component%20Object%20Reference) (OtherActor :type Actor%20Object%20Reference) (OtherComp :type Primitive%20Component%20Object%20Reference) (NormalImpulse :type Vector :default "0, 0, 0") (Hit :type Hit%20Result%20Structure%20%28by%20ref%29))
  ;[1 1 1] Enemy Bounce Player
  (bind _asbp_first_person_character (Utilities|Casting|CastToBP_FirstPersonCharacter OtherActor))
  (Character|LaunchCharacter _asbp_first_person_character (* (Math|Vector|GetUnitDirection(Vector) (Transformation|GetActorLocation) (Transformation|GetActorLocation _asbp_first_person_character)) 1.5e+03) false false))

(event OnComponentBeginOverlap(Capsule)
  (params (OverlappedComponent :type Primitive%20Component%20Object%20Reference) (OtherActor :type Actor%20Object%20Reference) (OtherComp :type Primitive%20Component%20Object%20Reference) (OtherBodyIndex :type Integer) (bFromSweep :type Boolean) (SweepResult :type Hit%20Result%20Structure%20%28by%20ref%29))
  ;[1 1 1] Enemy Hit from player
  (Utilities|Casting|CastToBP_FirstPersonCharacter OtherActor
    (:CastFailed
      (if (> (Math|Vector|VectorLength (Transformation|GetComponentVelocity OtherComp)) (Variables|Default|GetThresholdVelocity))
        (Game|Damage|ApplyDamage self 1e+02 0 0)
        (if (<= (Variables|Default|GetEnemyHealth) 0.0)
          (CallFunction|DropLoot))))))

(event Custom|FollowPlayer
  ;[1 1 1] Enemy Movement Animation
  (Variables|Default|SetcanAttack? true)
  (if (Variables|Default|GetisSeeingPlayer?)
    (AI|AIMoveTo self "0, 0, 0" (Game|GetPlayerCharacter 0) 2e+01 false
      (:OnSuccess
        (if (Variables|Default|GetcanAttack?)
          (Variables|Default|SetcanAttack? false)
          (bind _returnvalue (Animation|PlayAnimMontage "/Game/Animations/AI/Paired_CounterPunch_PalmStrike_Att_UE5_Montage.Paired_CounterPunch_PalmStrike_Att_UE5_Montage" 1.0 "None"))
          (Utilities|FlowControl|Delay _returnvalue)
          (Variables|Default|SetcanAttack? true))))
    (else
      (Variables|Default|SetisSeeingPlayer? false))))

(event Custom|Drop%20Loot
  (bind _returnvalue (Transformation|GetActorLocation))
  (bind _spawnertype (Variables|Default|GetspawnerType))
  ;[1 1 1] Comment
  (bind _outhit (Collision|LineTraceByChannel _returnvalue (- _returnvalue "0.000000,0.000000,200.000000") "TraceTypeQuery1" false (Utilities|Array|MakeArray (Game|GetPlayerCharacter 0)) "None"))
  (bind _returnvalue_2 (Game|SpawnActorfromClass (Utilities|Select :Index (Math|Random|RandomInteger 2) :Option%200 "/Game/Blueprints/Blocks/Block_Cube.Block_Cube_C" :Option%201 "/Game/Blueprints/Blocks/Block_Parallelogram.Block_Parallelogram_C" :Option%202 "/Game/Blueprints/Blocks/Block_Trapezium.Block_Trapezium_C" :Option%203 "/Game/Blueprints/Blocks/Block_Triangle.Block_Triangle_C") (Math|Transform|MakeTransform (.Location (Collision|BreakHitResult _outhit)) (Math|Rotator|MakeRotator 0.0 0.0 (Math|Random|RandomFloatinRange 0.0 0.0))) "Undefined" "MultiplyWithRoot" 0 0))
  (bind _asblock_cube (Utilities|Casting|CastToBlock_Cube _returnvalue_2)
    (:then
      (Default|ChangeMat _asblock_cube _spawnertype))
    (:CastFailed
      (bind _asblock_parallelogram (Utilities|Casting|CastToBlock_Parallelogram _returnvalue_2)
        (:then
          (Default|ChangeMat _asblock_parallelogram _spawnertype))
        (:CastFailed
          (bind _asblock_trapezium (Utilities|Casting|CastToBlock_Trapezium _returnvalue_2)
            (:then
              (Default|ChangeMat _asblock_trapezium _spawnertype))
            (:CastFailed
              (bind _asblock_triangle (Utilities|Casting|CastToBlock_Triangle _returnvalue_2))
              (Default|ChangeMat _asblock_triangle _spawnertype))))))))

(event EventTick
  (params (DeltaSeconds :type Float%20%28single-precision%29))
  ;[1 1 1] Enemy Follow Algorithm
  (if (not (Variables|Default|GetisSeeingPlayer?))
    (Components|Movement|StopMovementImmediately (Variables|Character|GetCharacterMovement))))

(event Game|Damage|EventAnyDamage
  (params (Damage :type Float%20%28single-precision%29) (DamageType :type Damage%20Type%20Object%20Reference) (InstigatedBy :type Controller%20Object%20Reference) (DamageCauser :type Actor%20Object%20Reference))
  ;[1 1 1] Enemy Health
  (Audio|PlaySound2D "/Game/Audio/SFX/enemyhit.enemyhit" 1.0 1.0 0.0 0 0)
  (Variables|Default|SetEnemyHealth (- (Variables|Default|GetEnemyHealth) Damage))
  (if (<= (Variables|Default|GetEnemyHealth) 0.0)
    (Actor|DestroyActor)))

(fn ConstructionScript)